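; Sleeping polar bear hazard that grows angrier while disturbed by the penguin player and triggers the Game_Over widget.
; Proximity overlap starts annoyance, and leaving clears it unless HearsASound is set.
; Tick drains AnnoyanceScale while annoyed and refills it otherwise, switching mesh, Zzz effect and anger material by threshold.
; Touching the bear or emptying the meter ends the game; debug printing remains, and the multiplier decay logic never runs.
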(event `self.ReceiveBeginPlay`)

(event `self.CloseToBearCollision.OnComponentBeginOverlap`
  (params (OverlappedComponent :type "PrimitiveComponent Object Reference") (OtherActor :type "Actor Object Reference") (OtherComp :type "PrimitiveComponent Object Reference") (OtherBodyIndex :type Integer) (bFromSweep :type Boolean) (SweepResult :type "HitResult Structure (by ref)"))
  (cast `/Game/MainLevel/BP_PenguinPlayer` OtherActor)
  (if (not (`self.IsCloseToBear`))
    (set `self.IsCloseToBear` true)
    (set `self.IsAnnoyingBear` true)
    (`StaticMeshComponent.SetStaticMesh` (`self.c_polarbear_a01`) "/Game/Characters/Polarbear/Meshes/c_polarbear_a02.c_polarbear_a02")
    (`ActorComponent.SetActive` (`self.Zzz___`) false false)
    (`GameplayStatics.PlaySound2D` "/Game/WorkingFolders/Sybren/SC_FX_Bear_Stage_01.SC_FX_Bear_Stage_01" 1.0 1.0 0.0 null null)))

(event `self.CloseToBearCollision.OnComponentEndOverlap`
  (params (OverlappedComponent :type "PrimitiveComponent Object Reference") (OtherActor :type "Actor Object Reference") (OtherComp :type "PrimitiveComponent Object Reference") (OtherBodyIndex :type Integer))
  (cast `/Game/MainLevel/BP_PenguinPlayer` OtherActor)
  (if (`self.IsCloseToBear`)
    (set `self.IsCloseToBear` false)
    (if (not (`self.HearsASound`))
      (set `self.IsAnnoyingBear` false)
      (`StaticMeshComponent.SetStaticMesh` (`self.c_polarbear_a01`) "/Game/Characters/Polarbear/Meshes/c_polarbear_a01.c_polarbear_a01")
      (`ActorComponent.SetActive` (`self.Zzz___`) true false))))

(event `self.TouchingBearCollision.OnComponentBeginOverlap`
  (params (OverlappedComponent :type "PrimitiveComponent Object Reference") (OtherActor :type "Actor Object Reference") (OtherComp :type "PrimitiveComponent Object Reference") (OtherBodyIndex :type Integer) (bFromSweep :type Boolean) (SweepResult :type "HitResult Structure (by ref)"))
  (cast `/Game/MainLevel/BP_PenguinPlayer` OtherActor)
  (`/Engine/EditorBlueprintResources/StandardMacros.DoOnce` false
    (:`Completed`
      (`GameplayStatics.PlaySound2D` "/Game/WorkingFolders/Sybren/SC_FX_Bear_Stage_04.SC_FX_Bear_Stage_04" 1.0 1.0 0.0 null null)
      (bind _returnvalue (`|CreateWidget` "/Game/WorkingFolders/Rahul/Level/Game_Over.Game_Over_C"))
      (`UserWidget.AddToViewport` _returnvalue 0)
      (set `PlayerController.bShowMouseCursor` true (`GameplayStatics.GetPlayerController` 0)))))

(event `self.ReceiveTick`
  (params (DeltaSeconds :type "Float (single-precision)"))
  (bind _annoyancescale (`self.AnnoyanceScale`))
  (if (`self.IsAnnoyingBear`)
    (if (<= (`self.AnnoyanceScale`) 0.0)
      (`/Engine/EditorBlueprintResources/StandardMacros.DoOnce` false
        (:`Completed`
          (`GameplayStatics.PlaySound2D` "/Game/WorkingFolders/Sybren/SC_FX_Bear_Stage_04.SC_FX_Bear_Stage_04" 1.0 1.0 0.0 null null)
          (bind _returnvalue (`|CreateWidget` "/Game/WorkingFolders/Rahul/Level/Game_Over.Game_Over_C"))
          (`UserWidget.AddToViewport` _returnvalue 0)
          (set `PlayerController.bShowMouseCursor` true (`GameplayStatics.GetPlayerController` 0))))
      (else
        (set `self.AnnoyanceScale` (- (`self.AnnoyanceScale`) DeltaSeconds))
        (`KismetSystemLibrary.PrintString` (`KismetStringLibrary.Conv_DoubleToString` _annoyancescale) :!label _label)
        (if (< _annoyancescale 8.0)
          (`StaticMeshComponent.SetStaticMesh` (`self.c_polarbear_a01`) "/Game/Characters/Polarbear/Meshes/c_polarbear_a02.c_polarbear_a02")
          (`ActorComponent.SetActive` (`self.Zzz___`) false false)
          (if (< (`self.AnnoyanceScale`) 5.0)
            (if (< (`self.AnnoyanceScale`) 2.0)
              (if (!= (`self.AnnoyanceStage`) 3)
                (`PrimitiveComponent.SetMaterial` (`self.c_polarbear_a01`) 0 "/Game/MainLevel/Bear/BearMaterials/BigMadBear.BigMadBear")
                (set `self.AnnoyanceStage` 3)
                (`GameplayStatics.PlaySound2D` "/Game/WorkingFolders/Sybren/SC_FX_Bear_Stage_02.SC_FX_Bear_Stage_02" 1.0 1.0 0.0 null null))
              (elif (!= (`self.AnnoyanceStage`) 2)
                (`PrimitiveComponent.SetMaterial` (`self.c_polarbear_a01`) 0 "/Game/MainLevel/Bear/BearMaterials/MidMadBear.MidMadBear")
                (set `self.AnnoyanceStage` 2)))
            (elif (!= (`self.AnnoyanceStage`) 1)
              (`PrimitiveComponent.SetMaterial` (`self.c_polarbear_a01`) 0 "/Game/MainLevel/Bear/BearMaterials/SmallMadBear.SmallMadBear")
              (set `self.AnnoyanceStage` 1)))
          (elif (!= (`self.AnnoyanceStage`) 0)
            (`StaticMeshComponent.SetStaticMesh` (`self.c_polarbear_a01`) "/Game/Characters/Polarbear/Meshes/c_polarbear_a01.c_polarbear_a01")
            (`ActorComponent.SetActive` (`self.Zzz___`) true false)
            (`PrimitiveComponent.SetMaterial` (`self.c_polarbear_a01`) 0 "/Game/Characters/Polarbear/Materials/polarbear.polarbear")
            (set `self.AnnoyanceStage` 0)))))
    (elif (>= (`self.AnnoyanceScale`) 10.0)
      (goto _label)
      (else
        (set `self.AnnoyanceScale` (+ (`self.AnnoyanceScale`) DeltaSeconds))
        (goto _label)))))

(fn `UserConstructionScript`)