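; Breakable ice tile actor that cracks under repeated hits and disappears when its lives run out.
; BeginPlay sets the life count and passes its mesh and bear-tile flag to the IceTile object.
; Each damage event costs one life regardless of amount, swapping crack materials by stage and hiding a secondary mesh early on.
; On breaking, it disables collision, plays a sound and triggers a victory check through the damage causer's IceBlocksManagement component.
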(event `self.ReceiveBeginPlay`
  (set `self.LivesAmount` 10)
  (add `self.OnTakeAnyDamage` (delegate `OnTakeAnyDamage_Event`))
  (set `IceTile.MeshComponent` (`self.IceBlockStaticBody`) (`self.IceTile`))
  (set `IceTile.IsBearBlock` (`self.isBearTile`) (`self.IceTile`)))

(event `OnTakeAnyDamage_Event` :!signature `self.OnTakeAnyDamage`
  (params (DamagedActor :type "Actor Object Reference") (Damage :type "Float (single-precision)") (DamageType :type "DamageType Object Reference") (InstigatedBy :type "Controller Object Reference") (DamageCauser :type "Actor Object Reference"))
  (bind _iceblockstaticbody (`self.IceBlockStaticBody`))
  (if (`self.isBreakable`)
    (bind _output_get (set `self.LivesAmount` (- (`self.LivesAmount`) 1)))
    (if (`IceTile.IsLivingBlock` (`self.IceTile`))
      (switch `int` _output_get
        (:`0`
          (`SceneComponent.SetVisibility` _iceblockstaticbody false true)
          (`PrimitiveComponent.SetCollisionEnabled` _iceblockstaticbody "NoCollision")
          (`GameplayStatics.PlaySound2D` "/Game/WorkingFolders/Sybren/SC_FX_Icebreak.SC_FX_Icebreak" 1.0 1.0 0.0 null null)
          (set `IceTile.IsLivingBlock` false (`self.IceTile`))
          (`IceBlocksManagement.TriggerVictoryCheck` (`self.GetComponentByClass` DamageCauser "/Script/ClimaxGameJam.IceBlocksManagement") (`self.K2_GetActorLocation`)))
        (:`1`
          (`PrimitiveComponent.SetMaterial` (`self.IceBlockStaticBody`) 0 "/Game/MainLevel/IceBlocks/IceBlockMaterials/IceMacroCrackMat.IceMacroCrackMat" :!label _label))
        (:`2`
          (goto _label))
        (:`3`
          (goto _label))
        (:`4`
          (`PrimitiveComponent.SetMaterial` (`self.IceBlockStaticBody`) 0 "/Game/WorkingFolders/Mag/Level/MagsMatrerials/IceMiniCrackMat.IceMiniCrackMat" :!label _label_2))
        (:`5`
          (goto _label_2))
        (:`6`
          (goto _label_2))
        (:`7`
          (`PrimitiveComponent.SetMaterial` (`self.IceBlockStaticBody`) 0 "/Game/WorkingFolders/Ythen/Materials/Ice/M_Ice_Inst.M_Ice_Inst" :!label _label_3)
          (if (`SceneComponent.IsVisible` (`self.StaticMesh1`))
            (`SceneComponent.SetVisibility` (`self.StaticMesh1`) false false)))
        (:`8`
          (goto _label_3))
        (:`9`
          (goto _label_3))
        (:`10`
          (goto _label_3))))))

(fn `UserConstructionScript`)