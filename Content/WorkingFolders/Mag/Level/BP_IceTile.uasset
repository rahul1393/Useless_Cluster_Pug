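; BP_IceTile is a breakable ice block that cracks progressively as it takes hits.
; When breakable, each damage event removes one of ten lives set at BeginPlay, regardless of damage amount.
; While the block is living, the remaining count selects intact, mid-crack or heavy-crack material, and early hits also hide a second mesh.
; At zero it hides the main mesh, disables its collision and plays a break sound.
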(event `self.ReceiveBeginPlay`
  (set `self.LivesAmount` 10)
  (add `self.OnTakeAnyDamage` (delegate `OnTakeAnyDamage_Event`)))

(event `OnTakeAnyDamage_Event` :!signature `self.OnTakeAnyDamage`
  (params (DamagedActor :type "Actor Object Reference") (Damage :type "Float (single-precision)") (DamageType :type "DamageType Object Reference") (InstigatedBy :type "Controller Object Reference") (DamageCauser :type "Actor Object Reference"))
  (bind _staticmesh (`self.StaticMesh`))
  (if (`self.isBreakable`)
    (bind _output_get (set `self.LivesAmount` (- (`self.LivesAmount`) 1)))
    (if (`self.isLivingIceBlock`)
      (switch `int` _output_get
        (:`0`
          (`SceneComponent.SetVisibility` _staticmesh false true)
          (`PrimitiveComponent.SetCollisionEnabled` _staticmesh "NoCollision")
          (`GameplayStatics.PlaySound2D` "/Game/WorkingFolders/Sybren/SC_FX_Icebreak.SC_FX_Icebreak" 1.0 1.0 0.0 null null)
          (set `self.isLivingIceBlock` false))
        (:`1`
          (`PrimitiveComponent.SetMaterial` (`self.StaticMesh`) 0 "/Game/WorkingFolders/Mag/Level/IceMacroCrackMat.IceMacroCrackMat" :!label _label))
        (:`2`
          (goto _label))
        (:`3`
          (goto _label))
        (:`4`
          (`PrimitiveComponent.SetMaterial` (`self.StaticMesh`) 0 "/Game/WorkingFolders/Mag/Level/IceMidCrackMat.IceMidCrackMat" :!label _label_2))
        (:`5`
          (goto _label_2))
        (:`6`
          (goto _label_2))
        (:`7`
          (`PrimitiveComponent.SetMaterial` (`self.StaticMesh`) 0 "/Game/WorkingFolders/Ythen/Materials/Ice/M_Ice_Inst.M_Ice_Inst" :!label _label_3)
          (if (`SceneComponent.IsVisible` (`self.StaticMesh1`))
            (`SceneComponent.SetVisibility` (`self.StaticMesh1`) false false)))
        (:`8`
          (goto _label_3))
        (:`9`
          (goto _label_3))
        (:`10`
          (goto _label_3))))))

(fn `UserConstructionScript`)