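; Seals_BP is a pushable seal that the penguin player can move while holding interact.
; Each tick it reads the player's Interact flag to toggle physics simulation on MoveableSeal, regardless of overlap.
; Box overlaps set the Tick flag, which gates the player's pushing state; end overlap also sets it true for the player, so leaving doesn't clear it.
; Walk speed is set to the same value whether pushing or released.
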(event `self.ReceiveBeginPlay`
  (bind _asbp_penguin_player (cast `/Game/MainLevel/BP_PenguinPlayer` (`GameplayStatics.GetPlayerCharacter` 0)))
  (set `self.As BP Penguin Player` _asbp_penguin_player))

(event `self.Box Collison.OnComponentBeginOverlap`
  (params (OverlappedComponent :type "PrimitiveComponent Object Reference") (OtherActor :type "Actor Object Reference") (OtherComp :type "PrimitiveComponent Object Reference") (OtherBodyIndex :type Integer) (bFromSweep :type Boolean) (SweepResult :type "HitResult Structure (by ref)"))
  (if (== OtherActor (`self.As BP Penguin Player`))
    (set `self.Tick` true)
    (else
      (set `self.Tick` false))))

(event `self.Box Collison.OnComponentEndOverlap`
  (params (OverlappedComponent :type "PrimitiveComponent Object Reference") (OtherActor :type "Actor Object Reference") (OtherComp :type "PrimitiveComponent Object Reference") (OtherBodyIndex :type Integer))
  (if (== OtherActor (`self.As BP Penguin Player`))
    (set `self.Tick` true)
    (else
      (set `self.Tick` false))))

(event `self.ReceiveTick`
  (params (DeltaSeconds :type "Float (single-precision)"))
  (bind _as_bp_penguin_player (`self.As BP Penguin Player`))
  (bind _charactermovement (`Character.CharacterMovement` _as_bp_penguin_player))
  (if (`/Game/MainLevel/BP_PenguinPlayer.Interact` (`self.As BP Penguin Player`))
    (`PrimitiveComponent.SetSimulatePhysics` (`self.MoveableSeal`) true)
    (if (`self.Tick`)
      (set `/Game/MainLevel/BP_PenguinPlayer.IsPushing` true _as_bp_penguin_player)
      (set `CharacterMovementComponent.MaxWalkSpeed` 200.0 _charactermovement))
    (else
      (`PrimitiveComponent.SetSimulatePhysics` (`self.MoveableSeal`) false)
      (set `/Game/MainLevel/BP_PenguinPlayer.IsPushing` false _as_bp_penguin_player)
      (set `CharacterMovementComponent.MaxWalkSpeed` 200.0 _charactermovement))))

(fn `UserConstructionScript`)