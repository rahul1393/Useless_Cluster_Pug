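; BP_IceTile_2 is a breakable ice tile that cracks progressively as it takes damage, then disappears.
; Each damage event removes one of ten lives regardless of amount, swapping the mesh to small, medium or big crack materials.
; At zero lives the mesh is hidden and loses collision, but the actor remains.
; A self-damage-on-hit handler exists, but its binding never runs, so damage must come from elsewhere.
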(event `self.ReceiveBeginPlay`
  (set `self.isLivingIceBlock` true)
  (set `self.LivesAmount` 10)
  (add `self.OnTakeAnyDamage` (delegate `OnTakeAnyDamage_Event`)))

(event `OnActorHit_Event` :!signature `self.OnActorHit`
  (params (SelfActor :type "Actor Object Reference") (OtherActor :type "Actor Object Reference") (NormalImpulse :type "Vector Structure") (Hit :type "HitResult Structure (by ref)"))
  (`GameplayStatics.ApplyDamage` self 1.0 null null "/Engine/EngineDamageTypes/DmgTypeBP_Environmental.DmgTypeBP_Environmental_C"))

(event `OnTakeAnyDamage_Event` :!signature `self.OnTakeAnyDamage`
  (params (DamagedActor :type "Actor Object Reference") (Damage :type "Float (single-precision)") (DamageType :type "DamageType Object Reference") (InstigatedBy :type "Controller Object Reference") (DamageCauser :type "Actor Object Reference"))
  (bind _staticmesh (`self.StaticMesh`))
  (bind _output_get (set `self.LivesAmount` (- (`self.LivesAmount`) 1)))
  (if (`self.isLivingIceBlock`)
    (switch `int` _output_get
      (:`0`
        (`SceneComponent.SetVisibility` _staticmesh false true)
        (`PrimitiveComponent.SetCollisionEnabled` _staticmesh "NoCollision")
        (set `self.isLivingIceBlock` false))
      (:`1`
        (`PrimitiveComponent.SetMaterial` _staticmesh 0 "/Game/WorkingFolders/Mag/Level/MagsMatrerials/IceBigCrackMat.IceBigCrackMat" :!label _label))
      (:`2`
        (goto _label))
      (:`3`
        (goto _label))
      (:`4`
        (`PrimitiveComponent.SetMaterial` _staticmesh 0 "/Game/WorkingFolders/Mag/Level/MagsMatrerials/IceMediumCrackMat.IceMediumCrackMat" :!label _label_2))
      (:`5`
        (goto _label_2))
      (:`6`
        (goto _label_2))
      (:`7`
        (`PrimitiveComponent.SetMaterial` _staticmesh 0 "/Game/WorkingFolders/Mag/Level/MagsMatrerials/IceSmallCrackMat.IceSmallCrackMat" :!label _label_3))
      (:`8`
        (goto _label_3))
      (:`9`
        (goto _label_3))
      (:`10`
        (`PrimitiveComponent.SetMaterial` _staticmesh 0 "/Game/WorkingFolders/Ythen/Materials/Ice/M_Ice_Inst.M_Ice_Inst")))))

(fn `UserConstructionScript`)